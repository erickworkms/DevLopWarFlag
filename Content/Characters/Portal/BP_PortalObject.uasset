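; BP_PortalObject is a portal actor whose appearance reflects a team selection.
; SetPortalMaterial passes the team to SetPortalMaterialMult, which switches on it and applies a colored material instance to the first slot of NPCLocalReference.
; Clients and Agile share blue, while Cascade gets red and No Job gets green.
; The construction script and default lifecycle events are empty.
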(event Custom|SetPortalMaterialMult
  (params (Selection :type ETeam%20Enum :default "Clients"))
  (switch Utilities|FlowControl|Switch|SwitchonETeam Selection
    (:Clients
      (Rendering|Material|SetMaterial (Variables|Default|GetNPCLocalReference) 0 "/Game/Characters/Portal/BlueMaterialPortalMaterial_Inst.BlueMaterialPortalMaterial_Inst"))
    (:Agile
      (Rendering|Material|SetMaterial (Variables|Default|GetNPCLocalReference) 0 "/Game/Characters/Portal/BlueMaterialPortalMaterial_Inst.BlueMaterialPortalMaterial_Inst"))
    (:Cascade
      (Rendering|Material|SetMaterial (Variables|Default|GetNPCLocalReference) 0 "/Game/Characters/Portal/RedMaterialPortalMaterial_Inst.RedMaterialPortalMaterial_Inst"))
    (:NoJob
      (Rendering|Material|SetMaterial (Variables|Default|GetNPCLocalReference) 0 "/Game/Characters/Portal/GreenMaterialPortalMaterial_Inst.GreenMaterialPortalMaterial_Inst"))))

(event EventBeginPlay)

(event Collision|EventActorBeginOverlap
  (params (OtherActor :type Actor%20Object%20Reference)))

(event EventTick
  (params (DeltaSeconds :type Float%20%28single-precision%29)))

(event EventSetPortalMaterial
  (params (team :type ETeam%20Enum :default "Clients"))
  (CallFunction|SetPortalMaterialMult team))

(fn ConstructionScript)